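; BP_FinishLine is the finish line actor that counts laps for karts crossing it.
; On overlap it casts to BP_Kart and checks track progress, incrementing Laps on success and calling OnLapProgress only for player 0's kart.
; A failed check goes through a DoOnce that decrements Laps, re-armed by any valid crossing; this gate is shared by all karts rather than tracked per kart.
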(event Collision|EventActorBeginOverlap
  (params (OtherActor :type Actor%20Object%20Reference))
  (bind _asbp_kart (Utilities|Casting|CastToBP_Kart OtherActor))
  (if (Default|GetTrackProgress _asbp_kart)
    (bind _result (Math|Integer|IncrementInt (Variables|/Game/Levels/Anuj/funWorld/BP_Kart.BP_Kart_C|GetLaps _asbp_kart))
      (:%20%20
        (if (== _asbp_kart (Game|Player|GetPlayerPawn 0))
          (Default|CallOnLapProgress _result)
          (goto _label Reset)
          (else
            (goto _label Reset)))))
    (else
      (Utilities|FlowControl|DoOnce false :!label _label
        (:Completed
          (Math|Integer|DecrementInt (Variables|/Game/Levels/Anuj/funWorld/BP_Kart.BP_Kart_C|GetLaps _asbp_kart)))))))

(event EventTick
  (params (DeltaSeconds :type Float%20%28single-precision%29)))

(fn ConstructionScript)