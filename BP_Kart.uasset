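; Physics-driven racing kart for player or AI, which flags the world complete and loads planet select once the HUD lap count exceeds the required laps.
; Each tick, line traces at four wheels apply spring suspension, alongside per-wheel drive forces and torque steering.
; AI karts derive throttle and steering from the BP_Spline track, which also provides course progress and reset placement.
; Timers handle toppled resets and temporary speed boosts.
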(event Input|EnhancedActionEvents|EnhancedInputActionIA_Accelerate
  (params (ActionValue :type Float%20%28double-precision%29) (ElapsedSeconds :type Float%20%28double-precision%29) (TriggeredSeconds :type Float%20%28double-precision%29) (InputAction :type Input%20Action%20Object%20Reference :default "/Game/Levels/Anuj/funWorld/Inputs/IA_Accelerate.IA_Accelerate"))
  ;[0.15 0.15 0.15 0.5] Acceleration
  (Variables|Default|SetAccelerationInput (Math|Interpolation|FInterpTo (Variables|Default|GetAccelerationInput) (Math|Float|SelectFloat ActionValue (Variables|Default|GetAccelerationInput) (CallFunction|IsonGround)) (Utilities|Time|GetWorldDeltaSeconds) 0.5)))

(event Input|EnhancedActionEvents|EnhancedInputActionIA_Steering
  (params (ActionValue :type Float%20%28double-precision%29) (ElapsedSeconds :type Float%20%28double-precision%29) (TriggeredSeconds :type Float%20%28double-precision%29) (InputAction :type Input%20Action%20Object%20Reference :default "/Game/Levels/Anuj/funWorld/Inputs/IA_Steering.IA_Steering"))
  ;[0.15 0.15 0.15 0.5] Sterring
  (Class|PrimitiveComponent|AddTorqueinRadians (Variables|Default|GetBox_Collision) (Math|Vector|MakeVector 0.0 0.0 (* ActionValue (Variables|Default|GetSteeringTorque))) "None" false)
  (Transformation|SetRelativeRotation (Variables|Default|GetFL_Wheek) (Math|Rotator|MakeRotator 0.0 0.0 (Math|Interpolation|FInterpTo (.yaw (Variables|/Script/Engine.SceneComponent|GetRelativeRotation (Variables|Default|GetFL_Wheek))) ActionValue (Utilities|Time|GetWorldDeltaSeconds) 3.0)) false false))

(event EventBeginPlay
  ;[0.15 0.15 0.15 0.5] Game Start
  (Utilities|FlowControl|Delay 5.0)
  (Variables|Default|SetDelayComplete true)
  (Input|AddMappingContext (PlayerController|LocalPlayerSubsystems|GetEnhancedInputLocalPlayerSubsystem (Game|GetPlayerController 0)) "/Game/Levels/Anuj/funWorld/Inputs/IMC_Kart.IMC_Kart" 0 "(bIgnoreAllPressedKeysUntilRelease=True,bForceImmediately=False,bNotifyUserSettings=False)")
  (bind _returnvalue (Actor|GetActorOfClass "/Game/Levels/Anuj/funWorld/BP_Spline.BP_Spline_C"))
  (Variables|Default|SetTrack _returnvalue)
  (bind _returnvalue_2 (UserInterface|CreateWidget "/Game/Levels/Anuj/funWorld/UI/W_HUD.W_HUD_C"))
  (Variables|Default|SetHUD _returnvalue_2)
  (UserInterface|Viewport|AddtoViewport _returnvalue_2 0)
  (bind _asgm_kart (Utilities|Casting|CastToGM_Kart (Game|GetGameMode)))
  (Default|AddKart _asgm_kart self))

(event EventTick
  (params (DeltaSeconds :type Float%20%28single-precision%29))
  (bind _hud (Variables|Default|GetHUD))
  (bind _w_lapcount (Variables|/Game/Levels/Anuj/funWorld/UI/W_HUD.W_HUD_C|GetW_LapCount _hud))
  ;[0.15 0.15 0.15 0.5] Game Mechanics
  (if (Variables|Default|GetDelayComplete)
    (if (> (Math|Conversions|ToInteger(Byte) (Utilities|String|ToString(Text) (Class|TextBlock|GetText (Variables|/Game/Levels/Anuj/funWorld/UI/W_LapCount.W_LapCount_C|GetTXT_CurrentLap _w_lapcount)))) (Math|Conversions|ToInteger(Byte) (Utilities|String|ToString(Text) (Class|TextBlock|GetText (Variables|/Game/Levels/Anuj/funWorld/UI/W_LapCount.W_LapCount_C|GetTXT_RequiredLaps _w_lapcount)))))
      (bind _asgi_ashspire (Utilities|Casting|CastToGI_Ashspire (Game|GetGameInstance)))
      (Variables|/Game/Levels/Aakash/GI_Ashspire.GI_Ashspire_C|SetFunWorldComplete _asgi_ashspire true)
      (Game|OpenLevel(byName) "PlanetSelect_Level")
      (else
        (Utilities|FlowControl|Sequence
          (:then_0
            (CallFunction|SuspensionCast (Variables|Default|GetFL_Wheek))
            (CallFunction|SuspensionCast (Variables|Default|GetFR_Wheel))
            (CallFunction|SuspensionCast (Variables|Default|GetBR_Wheel))
            (CallFunction|SuspensionCast (Variables|Default|GetBL_Wheel))
            (CallFunction|CalculateAcceleration)
            (CallFunction|IsToppled)
            (Math|Float|CompareFloat (Variables|Default|GetAccelerationInput) 0.0))
          (:then_1
            (if (!= (Pawn|GetController) (Game|GetPlayerController 0))
              (CallFunction|AIAccelerateKart (CallFunction|GetAIThrottle))
              (CallFunction|AISteerKart (CallFunction|GetAISteering)))))))))

(fn ConstructionScript
  ;[0.15 0.15 0.15 0.5] Kart Appearence
  (bind _returnvalue (Rendering|Material|CreateDynamicMaterialInstance (Variables|Default|GetCube) 0 "/Game/Levels/Anuj/funWorld/M_KartBody_Inst.M_KartBody_Inst" "None" :!class /Script/Engine.PrimitiveComponent))
  (Rendering|Material|SetVectorParameterValue _returnvalue "Colour" (Variables|Default|GetDebugCol) :!class /Script/Engine.MaterialInstanceDynamic)
  (Rendering|Material|SetMaterial (Variables|Default|GetCube) 0 _returnvalue))

(fn SuspensionCast
  (params (WheelComp :type Scene%20Component%20Object%20Reference))
  (bind _returnvalue (Transformation|GetWorldLocation WheelComp))
  (bind _returnvalue_2 (Components|GetChildComponent WheelComp 0))
  ;[0.15 0.15 0.15 0.5] Suspension of Kart
  (bind _outhit (Collision|LineTraceByChannel _returnvalue (+ _returnvalue (* (Math|Vector|GetUpVector WheelComp) -6e+01)) "TraceTypeQuery1" false 0 "ForOneFrame"))
  (if (.bBlockingHit (Collision|BreakHitResult _outhit))
    (Class|PrimitiveComponent|AddForceatLocation (Variables|Default|GetBox_Collision) (* (- 1.0 (Math|Float|NormalizetoRange (.Distance (Collision|BreakHitResult _outhit)) 0.0 6e+01)) (Math|Vector|GetUnitDirection(Vector) (.TraceEnd (Collision|BreakHitResult _outhit)) (.TraceStart (Collision|BreakHitResult _outhit))) 9e+04) (Transformation|GetWorldLocation WheelComp) "None")
    (CallFunction|AccelerateKart WheelComp)
    (Transformation|SetRelativeLocation _returnvalue_2 (Math|Vector|MakeVector 0.0 0.0 (Math|Interpolation|FInterpTo (.z (Variables|/Script/Engine.SceneComponent|GetRelativeLocation _returnvalue_2)) (+ (* (.Distance (Collision|BreakHitResult _outhit)) -1.0) 2e+01) (Utilities|Time|GetWorldDeltaSeconds) 3.0)) false false)
    (else
      (CallFunction|AccelerateKart WheelComp))))

(fn CalculateAcceleration
  (bind _accelerationinput (Variables|Default|GetAccelerationInput))
  ;[0.15 0.15 0.15 0.5] Kart Acceleration
  (bind _output_get (Variables|Default|SetAcceleration (* (Math|Float|Lerp 0.0 (Variables|Default|GetMaxAcceleration) _accelerationinput) _accelerationinput)))
  (Variables|Default|SetAcceleration (Math|Interpolation|FInterpTo (Variables|Default|GetAccelerationInput) 0.0 (Utilities|Time|GetWorldDeltaSeconds) 0.3))
  (Transformation|AddLocalRotation (Variables|Default|GetWheel4) (Math|Rotator|MakeRotator 0.0 (/ _output_get -0.1) 0.0) false false)
  (Transformation|AddLocalRotation (Variables|Default|GetWheel1) (Math|Rotator|MakeRotator 0.0 (* _output_get 1e+01) 0.0) false false))

(fn AccelerateKart
  (params (WheelComp :type Scene%20Component%20Object%20Reference))
  (bind _box_collision (Variables|Default|GetBox_Collision))
  ;[0.15 0.15 0.15 0.5] Acceleration
  (Class|PrimitiveComponent|AddForceatLocation (Variables|Default|GetBox_Collision) (+ (* (Math|Vector|GetForwardVector _box_collision) 1.5e+03 (Variables|Default|GetAccelerationInput) (Physics|GetMass _box_collision) (Variables|Default|GetSpeedMod)) (Math|Vector|SelectVector "0, 0, 0" (Math|Vector|MakeVector 0.0 0.0 (Variables|Default|GetDownforce)) (CallFunction|IsonGround))) (Transformation|GetWorldLocation WheelComp) "None")
  (Class|PrimitiveComponent|SetCenterOfMass (Variables|Default|GetBox_Collision) (* "-25.000000,0.000000,0.000000" (Variables|Default|GetAccelerationInput)) "None"))

(fn IsonGround
  (bind _returnvalue (Transformation|GetActorLocation))
  ;[0.15 0.15 0.15 0.5] Kart Position
  (bind _returnvalue_2 (Collision|LineTraceByChannel _returnvalue (- _returnvalue "0.000000,0.000000,40.000000") "TraceTypeQuery1" false 0 "None"))
  (return _returnvalue_2))

(fn GetTrackProgress
  (bind _track (Variables|Default|GetTrack))
  (bind _spline (Variables|/Game/Levels/Anuj/funWorld/BP_Spline.BP_Spline_C|GetSpline _track))
  ;[0.15 0.15 0.15 0.5] Track Percentage completion
  (return (> (Math|Vector|DotProduct (Math|Vector|Normalize (Transformation|GetVelocity)) (Math|Vector|Normalize (Class|SplineComponent|GetDirectionatSplineInputKey _spline (Class|SplineComponent|FindInputKeyClosesttoWorldLocation _spline (Transformation|GetActorLocation)) "World"))) 0.0)))

(fn BoostKart
  (params (SpeedMod :type Float%20%28single-precision%29) (Time :type Float%20%28single-precision%29))
  ;[0.15 0.15 0.15 0.5] Boost Multiplier
  (Variables|Default|SetSpeedMod SpeedMod)
  (Utilities|Time|SetTimerbyFunctionName 0 "ResetSpeed" Time))

(fn ResetSpeed
  ;[0.15 0.15 0.15 0.5] Reset Speed after boost or restart
  (Variables|Default|SetSpeedMod 1.0))

(fn AIAccelerateKart
  (params (Throttle :type Float%20%28double-precision%29))
  ;[0.15 0.15 0.15 0.5] AI Acceleration
  (Variables|Default|SetAccelerationInput (Math|Interpolation|FInterpTo (Variables|Default|GetAccelerationInput) (Math|Float|SelectFloat Throttle (Variables|Default|GetAccelerationInput) (CallFunction|IsonGround)) (Utilities|Time|GetWorldDeltaSeconds) 0.5)))

(fn AISteerKart
  (params (A :type Float%20%28double-precision%29))
  ;[0.15 0.15 0.15 0.5] AI Steering
  (Class|PrimitiveComponent|AddTorqueinRadians (Variables|Default|GetBox_Collision) (Math|Vector|MakeVector 0.0 0.0 (* A (Variables|Default|GetSteeringTorque) (* (Variables|Default|GetAccelerationInput) 2.0))) "None" false)
  (Transformation|SetRelativeRotation (Variables|Default|GetFL_Wheek) (Math|Rotator|MakeRotator 0.0 0.0 (Math|Interpolation|FInterpTo (.yaw (Variables|/Script/Engine.SceneComponent|GetRelativeRotation (Variables|Default|GetFL_Wheek))) A (Utilities|Time|GetWorldDeltaSeconds) 3.0)) false false))

(fn GetAISteering
  (bind _returnvalue (Transformation|GetActorLocation))
  (bind _returnvalue_2 (Transformation|GetActorRightVector))
  (bind _returnvalue_3 (Transformation|GetActorForwardVector))
  (bind _track (Variables|Default|GetTrack))
  (bind _returnvalue_4 (* _returnvalue_3 5e+02))
  (bind _spline (Variables|/Game/Levels/Anuj/funWorld/BP_Spline.BP_Spline_C|GetSpline _track))
  (bind _returnvalue_5 (+ _returnvalue _returnvalue_4))
  (bind _returnvalue_6 (Spline|FindDirectionClosesttoWorldLocation _spline _returnvalue_5 "World"))
  (bind _returnvalue_7 (Math|Vector|DotProduct _returnvalue_6 _returnvalue_2))
  ;[0.15 0.15 0.15 0.5] AI Steering Direction
  (return (* _returnvalue_7 (Variables|Default|GetAcceleration) (Math|Float|Power (Math|Float|Absolute(Float) (+ _returnvalue_7 5.0)) 2.5))))

(fn GetAIThrottle
  (bind _returnvalue (Transformation|GetActorLocation))
  (bind _returnvalue_2 (Transformation|GetActorForwardVector))
  (bind _track (Variables|Default|GetTrack))
  (bind _spline (Variables|/Game/Levels/Anuj/funWorld/BP_Spline.BP_Spline_C|GetSpline _track))
  (bind _returnvalue_3 (Spline|FindDirectionClosesttoWorldLocation _spline _returnvalue "World"))
  (bind _returnvalue_4 (Math|Vector|DotProduct _returnvalue_3 _returnvalue_2))
  (return (* (Math|Float|Clamp(Float) (Math|Float|Absolute(Float) _returnvalue_4) 0.5) (Math|Float|Sign(Float) _returnvalue_4))))

(fn GetCourseProgress
  (bind _track (Variables|Default|GetTrack))
  (bind _spline (Variables|/Game/Levels/Anuj/funWorld/BP_Spline.BP_Spline_C|GetSpline _track))
  ;[0.15 0.15 0.15 0.5] Overall Progress
  (return (+ (/ (Class|SplineComponent|GetDistanceAlongSplineatLocation _spline (Spline|FindLocationClosesttoWorldLocation _spline (Transformation|GetActorLocation) "Local") "Local") (Spline|GetSplineLength _spline)) (Variables|Default|GetLaps))))

(fn IsToppled
  ;[0.15 0.15 0.15 0.5] Is Upside Down
  (if (and (< (Math|Vector|DotProduct (Transformation|GetActorUpVector) "0.000000,0.000000,1.000000") 0.8) (not (Utilities|Time|IsValidTimerHandle (Variables|Default|GetResetTimer))))
    (bind _returnvalue (Utilities|Time|SetTimerbyEvent (EventDispatchers|CreateEvent :!event ResetPosition) 3.5))
    (Variables|Default|SetResetTimer _returnvalue)))

(fn ResetPosition
  (bind _returnvalue (Transformation|GetActorLocation))
  (bind _track (Variables|Default|GetTrack))
  (bind _spline (Variables|/Game/Levels/Anuj/funWorld/BP_Spline.BP_Spline_C|GetSpline _track))
  ;[0.15 0.15 0.15 0.5] Reset if all wheels leave the track
  (Utilities|Time|ClearandInvalidateTimerbyHandle (Variables|Default|GetResetTimer))
  (Transformation|SetActorLocationAndRotation (Spline|FindLocationClosesttoWorldLocation _spline _returnvalue "World") (Math|Conversions|RotationFromXVector (Spline|FindDirectionClosesttoWorldLocation _spline _returnvalue "World")))
  (Variables|Default|SetAccelerationInput 0.0))

(fn AwardItem
  (params (Item :type DA%20Item%20Object%20Reference))
  ;[0.15 0.15 0.15 0.5] Get Item From Mysterybox
  (Variables|Default|SetItem Item))