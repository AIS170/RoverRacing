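; BP_Missile is a missile actor that destroys itself on hit and spawns an explosion particle effect at the impact location.
; Tick runs a debug-drawn visibility trace downward from just ahead of the missile, but nothing acts on the result.
; An unconnected plane-projection node is also present, and the graphs contain no movement or damage logic.
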(event EventBeginPlay)

(event Collision|EventActorBeginOverlap
  (params (OtherActor :type Actor%20Object%20Reference)))

(event EventTick
  (params (DeltaSeconds :type Float%20%28single-precision%29))
  (bind _returnvalue (Transformation|GetActorLocation))
  (bind _returnvalue_2 (Transformation|GetActorForwardVector))
  (bind _returnvalue_3 (* _returnvalue_2 5e+01))
  (bind _returnvalue_4 (+ _returnvalue _returnvalue_3))
  (bind (_outhit _returnvalue_5) (Collision|LineTraceByChannel _returnvalue_4 (+ _returnvalue_4 "0.000000,0.000000,-500.000000") "TraceTypeQuery1" false 0 "ForOneFrame"))
  (if _returnvalue_5
    _))

(event Collision|EventHit
  (params (MyComp :type Primitive%20Component%20Object%20Reference) (Other :type Actor%20Object%20Reference) (OtherComp :type Primitive%20Component%20Object%20Reference) (bSelfMoved :type Boolean) (HitLocation :type Vector :default "0, 0, 0") (HitNormal :type Vector :default "0, 0, 0") (NormalImpulse :type Vector :default "0, 0, 0") (Hit :type Hit%20Result%20Structure%20%28by%20ref%29))
  (Actor|DestroyActor)
  (Effects|SpawnEmitteratLocation "/Game/Shared/StarterContent/Particles/P_Explosion.P_Explosion" HitLocation))

(fn ConstructionScript
  (|CallParentFunction))